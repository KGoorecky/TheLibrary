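; Interactable fridge for level one that gives the player pierogi by setting HasPierogi on the level-one character.
; The hover event caches the player reference and toggles the interaction prompt while the player has no pierogi.
; Interacting runs once, granting the item, playing a fridge sound at the actor's location and hiding the prompt.
; IsInteractable always returns false.
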(event `/Game/Dynamic/Interfaces/IF_Interact.OnInteract`
  (params (InteractingPlayer :type "Character Object Reference"))
  (`/Engine/EditorBlueprintResources/StandardMacros.DoOnce` false
    (:`Completed`
      (set `/Game/Dynamic/Characters/LevelOne/BP_CharacterLevelOne.HasPierogi` true (stale `/Game/Dynamic/Interfaces/IF_Interact.OnHovered` _output_get))
      (`GameplayStatics.PlaySoundAtLocation` "/Game/Dynamic/MetaSound/Sounds/MS_Fridge.MS_Fridge" (`self.K2_GetActorLocation`) (struct) 1.0 1.0 0.0 null null null null)
      (`/Game/Dynamic/UI/WB_InteractPrompt.ToggleInteractionIndicator` (`/Game/Dynamic/Characters/LevelOne/BP_CharacterLevelOne.InteractPromptWidget` (stale `/Game/Dynamic/Interfaces/IF_Interact.OnHovered` PlayerRefLevelOne)) false))))

(event `/Game/Dynamic/Interfaces/IF_Interact.OnHovered`
  (params (IsHovered :type Boolean) (PlayerRefMC :type "/Game/Dynamic/Characters/MainCharacter/BP_MainCharacter Object Reference") (PlayerRefLevelOne :type "/Game/Dynamic/Characters/LevelOne/BP_CharacterLevelOne Object Reference"))
  (bind _output_get (set `self.CharacterLevelOne` PlayerRefLevelOne))
  (if (not (`/Game/Dynamic/Characters/LevelOne/BP_CharacterLevelOne.HasPierogi` _output_get))
    (`/Engine/EditorBlueprintResources/StandardMacros.IsValid` PlayerRefLevelOne
      (:`Is Valid`
        (`/Game/Dynamic/UI/WB_InteractPrompt.ToggleInteractionIndicator` (`/Game/Dynamic/Characters/LevelOne/BP_CharacterLevelOne.InteractPromptWidget` PlayerRefLevelOne) IsHovered)))))

(fn `IsInteractable`
  (returns (Interactable :type Boolean))
  (return false))

(fn `UserConstructionScript`)