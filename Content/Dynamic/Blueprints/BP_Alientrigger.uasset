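; Trigger volume actor that stages an alien ambush with a UFO and sound cues, and starts forest ambience on BeginPlay.
; Each player overlap of the box spawns five BT_alien-driven aliens at chained offsets ahead of the player.
; It then turns a random Test-interface actor's lights red and rotates it, provided it casts to BP_Lightalien.
; Only then does it spawn a UFO above the player and, after a delay, play pursuit audio.
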(event `self.ReceiveBeginPlay`
  (`GameplayStatics.PlaySound2D` "/Game/Dynamic/MetaSound/Sounds/MS_ForestAmbient.MS_ForestAmbient" 1.0 1.0 0.0 null null))

(event `self.Box.OnComponentBeginOverlap`
  (params (OverlappedComponent :type "PrimitiveComponent Object Reference") (OtherActor :type "Actor Object Reference") (OtherComp :type "PrimitiveComponent Object Reference") (OtherBodyIndex :type Integer) (bFromSweep :type Boolean) (SweepResult :type "HitResult Structure (by ref)"))
  (bind _returnvalue (`GameplayStatics.GetPlayerCharacter` 0))
  (bind _returnvalue_2 (+ (`self.K2_GetActorLocation` _returnvalue) (* (`self.GetActorForwardVector` _returnvalue) (1000.0 1000.0 100.0))))
  (bind _returnvalue_3 (+ _returnvalue_2 (500.0 500.0 0.0)))
  (bind _returnvalue_4 (+ _returnvalue_3 (-100.0 200.0 0.0)))
  (bind _returnvalue_5 (+ _returnvalue_4 (200.0 100.0 0.0)))
  (if (== OtherActor (`GameplayStatics.GetPlayerCharacter` 0))
    (`GameplayStatics.PlaySound2D` "/Game/Dynamic/MetaSound/Sounds/MS_UFO.MS_UFO" 1.0 1.0 0.0 null null)
    (`AIBlueprintHelperLibrary.SpawnAIFromClass` "/Game/Dynamic/Characters/NPCs/BP_Alien.BP_Alien_C" "/Game/Dynamic/AI/NPC1/BT_alien.BT_alien" _returnvalue_2 (struct :`Yaw` 180.0) false null)
    (`AIBlueprintHelperLibrary.SpawnAIFromClass` "/Game/Dynamic/Characters/NPCs/BP_Alien.BP_Alien_C" "/Game/Dynamic/AI/NPC1/BT_alien.BT_alien" _returnvalue_3 (struct :`Yaw` 180.0) false null)
    (`AIBlueprintHelperLibrary.SpawnAIFromClass` "/Game/Dynamic/Characters/NPCs/BP_Alien.BP_Alien_C" "/Game/Dynamic/AI/NPC1/BT_alien.BT_alien" _returnvalue_4 (struct :`Yaw` 180.0) false null)
    (`AIBlueprintHelperLibrary.SpawnAIFromClass` "/Game/Dynamic/Characters/NPCs/BP_Alien.BP_Alien_C" "/Game/Dynamic/AI/NPC1/BT_alien.BT_alien" _returnvalue_5 (struct :`Yaw` 180.0) false null)
    (`AIBlueprintHelperLibrary.SpawnAIFromClass` "/Game/Dynamic/Characters/NPCs/BP_Alien.BP_Alien_C" "/Game/Dynamic/AI/NPC1/BT_alien.BT_alien" (+ _returnvalue_5 (0.0 100.0 0.0)) (struct :`Yaw` 180.0) false null)
    (bind _outactors (`GameplayStatics.GetAllActorsWithInterface` "/Game/Dynamic/Interfaces/test.test_C"))
    (bind _asbp_lightalien (cast `/Game/Dynamic/Blueprints/BP_Lightalien` (`KismetArrayLibrary.Array_Random` _outactors)))
    (`LightComponent.SetLightColor` (`/Game/Dynamic/Blueprints/BP_Lightalien.SpotLight` _asbp_lightalien) (`KismetMathLibrary.LinearColor_Red`) true)
    (`LightComponent.SetLightColor` (`/Game/Dynamic/Blueprints/BP_Lightalien.PointLight` _asbp_lightalien) (`KismetMathLibrary.LinearColor_Red`) true)
    (`self.K2_SetActorRotation` _asbp_lightalien (struct :`Yaw` -120.0) false)
    (`AIBlueprintHelperLibrary.SpawnAIFromClass` "/Game/Dynamic/Characters/NPCs/BP_UFO.BP_UFO_C" null (+ (`self.K2_GetActorLocation` (`GameplayStatics.GetPlayerCharacter` 0)) (0.0 0.0 200.0)) (struct) false null)
    (`KismetSystemLibrary.Delay` 6.5)
    (`GameplayStatics.PlaySound2D` "/Game/Dynamic/MetaSound/Music/MS_AlienPursuit.MS_AlienPursuit" 1.0 1.0 0.0 null null)))

(fn `UserConstructionScript`)