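; BP_sOMSIAD is a neighbour actor whose appearance and behaviour depend on the day count from BP_Wyjsciedopracy.
; On BeginPlay, days 0–3 start a timeline that shifts it along X and hides the mesh when finished, with early days swapping the mesh.
; Player overlap triggers an interaction and stops the timeline.
; On day 4, the interaction teleports the player to the Piwnica (cellar) actor, then plays the timeline after a delay.
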(event `self.ReceiveBeginPlay`
  (bind (_returnvalue_x _returnvalue_y _returnvalue_z) (`KismetMathLibrary.BreakVector` (`self.K2_GetActorLocation`)))
  (bind _cone (`self.Cone`))
  (bind _returnvalue (`GameplayStatics.GetActorOfClass` "/Game/Dynamic/Blueprints/BP_Wyjsciedopracy.BP_Wyjsciedopracy_C"))
  (switch `int` (`/Game/Dynamic/Blueprints/BP_Wyjsciedopracy.daycount` _returnvalue)
    (:`0`
      (`StaticMeshComponent.SetStaticMesh` _cone "/Engine/BasicShapes/Cylinder.Cylinder")
      (bind (_direction _track1) (`Timeline|Idzie` :!label _label)
        (:`Update`
          (`self.K2_SetActorLocation` (`KismetMathLibrary.MakeVector` (- _returnvalue_x _track1) _returnvalue_y _returnvalue_z)))
        (:`Finished`
          (`SceneComponent.SetVisibility` (`self.Cone`) false false))))
    (:`1`
      (`StaticMeshComponent.SetStaticMesh` _cone "/Engine/BasicShapes/Cube.Cube")
      (goto _label))
    (:`2`
      (`StaticMeshComponent.SetStaticMesh` _cone "/Game/Static/Meshes/lesosna/sosenka.sosenka")
      (goto _label))
    (:`3`
      (goto _label))))

(event `canibal`
  (bind _returnvalue (`GameplayStatics.GetActorOfClass` "/Game/Dynamic/Blueprints/piwnica.piwnica_C"))
  (`self.K2_SetActorLocation` (`GameplayStatics.GetPlayerCharacter` 0) (`self.K2_GetActorLocation` _returnvalue) false false))

(event `koniec interakcji`
  (goto _label))

(event `self.Box.OnComponentBeginOverlap`
  (params (OverlappedComponent :type "PrimitiveComponent Object Reference") (OtherActor :type "Actor Object Reference") (OtherComp :type "PrimitiveComponent Object Reference") (OtherBodyIndex :type Integer) (bFromSweep :type Boolean) (SweepResult :type "HitResult Structure (by ref)"))
  (if (== OtherActor (`GameplayStatics.GetPlayerCharacter` 0))
    (`|ExecutionSequence`
      (:`then_0`
        (`self.Interakcja`))
      (:`then_1`
        (goto _label :!via `Stop`)))))

(event `Interakcja`
  (if (== (`/Game/Dynamic/Blueprints/BP_Wyjsciedopracy.daycount` (stale `self.ReceiveBeginPlay` _returnvalue)) 4)
    (`self.canibal`)
    (`KismetSystemLibrary.Delay` 2.0)
    (`self.koniec interakcji`)
    (else
      (`self.koniec interakcji`))))

(fn `UserConstructionScript`)