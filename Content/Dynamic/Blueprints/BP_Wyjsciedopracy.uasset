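; BP_Wyjsciedopracy ("exit to work") is a trigger that advances the day and sends the player to the apartment.
; When the player character overlaps its Box, a switch on Daycount routes days 0 to 3 into one shared branch.
; That branch increments and prints Daycount, then moves the player to the location of the Apartament actor found by class.
; Other day values have no handling.
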(event `self.Box.OnComponentBeginOverlap`
  (params (OverlappedComponent :type "PrimitiveComponent Object Reference") (OtherActor :type "Actor Object Reference") (OtherComp :type "PrimitiveComponent Object Reference") (OtherBodyIndex :type Integer) (bFromSweep :type Boolean) (SweepResult :type "HitResult Structure (by ref)"))
  (if (== OtherActor (`GameplayStatics.GetPlayerCharacter` 0))
    (switch `int` (`self.daycount`)
      (:`0`
        _)
      (:`1`
        _)
      (:`2`
        _)
      (:`3`
        _))
    (bind _result (`/Engine/EditorBlueprintResources/StandardMacros.IncrementInt` (`self.daycount`))
      (:`  `
        (`KismetSystemLibrary.PrintString` (`KismetStringLibrary.Conv_IntToString` _result))
        (bind _returnvalue (`GameplayStatics.GetActorOfClass` "/Game/Dynamic/Blueprints/apartament.apartament_C"))
        (`self.K2_SetActorLocation` (`GameplayStatics.GetPlayerCharacter` 0) (`self.K2_GetActorLocation` _returnvalue) false false)))))

(fn `UserConstructionScript`)