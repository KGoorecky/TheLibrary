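; BP_Piwo is a level-one interactable beer pickup that the player collects, affecting the standing detective.
; Hovering caches the player and toggles its interaction prompt while HasPiwo is unset.
; Interacting sets HasPiwo on player and game instance, enables detective visibility there and calls SetVisibilityMessage on BP_DetectiveStanding actors.
; It then plays a sound, hides the prompt and destroys itself; IsInteractable always returns false.
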(event `/Game/Dynamic/Interfaces/IF_Interact.OnInteract`
  (params (InteractingPlayer :type "Character Object Reference"))
  (set `/Game/Dynamic/Characters/LevelOne/BP_CharacterLevelOne.HasPiwo` true (stale `/Game/Dynamic/Interfaces/IF_Interact.OnHovered` _output_get))
  (bind _outactors (`GameplayStatics.GetAllActorsOfClass` "/Game/Dynamic/Characters/NPCs/BP_Detective-Standing.BP_Detective-Standing_C"))
  (message `/Game/Dynamic/Interfaces/IF_Interact.SetVisibility` _outactors true)
  (bind _asgi_instance (cast `/Game/Dynamic/GI_Instance` (`GameplayStatics.GetGameInstance`)))
  (set `/Game/Dynamic/GI_Instance.HasPiwo` true _asgi_instance)
  (set `/Game/Dynamic/GI_Instance.DetectiveVisibility` true _asgi_instance)
  (`GameplayStatics.PlaySoundAtLocation` "/Game/Dynamic/MetaSound/Sounds/MS_Piwo.MS_Piwo" (`self.K2_GetActorLocation`) (struct) 1.0 1.0 0.0 null null null null)
  (`/Game/Dynamic/UI/WB_InteractPrompt.ToggleInteractionIndicator` (`/Game/Dynamic/Characters/LevelOne/BP_CharacterLevelOne.InteractPromptWidget` (stale `/Game/Dynamic/Interfaces/IF_Interact.OnHovered` PlayerRefLevelOne)) false)
  (`self.K2_DestroyActor`))

(event `/Game/Dynamic/Interfaces/IF_Interact.OnHovered`
  (params (IsHovered :type Boolean) (PlayerRefMC :type "/Game/Dynamic/Characters/MainCharacter/BP_MainCharacter Object Reference") (PlayerRefLevelOne :type "/Game/Dynamic/Characters/LevelOne/BP_CharacterLevelOne Object Reference"))
  (bind _output_get (set `self.CharacterLevelOne` PlayerRefLevelOne))
  (if (not (`/Game/Dynamic/Characters/LevelOne/BP_CharacterLevelOne.HasPiwo` _output_get))
    (`/Engine/EditorBlueprintResources/StandardMacros.IsValid` PlayerRefLevelOne
      (:`Is Valid`
        (`/Game/Dynamic/UI/WB_InteractPrompt.ToggleInteractionIndicator` (`/Game/Dynamic/Characters/LevelOne/BP_CharacterLevelOne.InteractPromptWidget` PlayerRefLevelOne) IsHovered)))))

(fn `IsInteractable`
  (returns (Interactable :type Boolean))
  (return false))

(fn `UserConstructionScript`)