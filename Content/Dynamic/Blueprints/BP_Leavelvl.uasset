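; BP_Leavelvl is a level-exit trigger that sends the player to MAP_Library.
; When the player character first overlaps its Box, a DoOnce plays the MS_PolonezStartUp sound, disables pawn input and starts a camera fade-out.
; After a delay matching the fade duration, it re-enables input and opens the library map by name.
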(event `self.Box.OnComponentBeginOverlap`
  (params (OverlappedComponent :type "PrimitiveComponent Object Reference") (OtherActor :type "Actor Object Reference") (OtherComp :type "PrimitiveComponent Object Reference") (OtherBodyIndex :type Integer) (bFromSweep :type Boolean) (SweepResult :type "HitResult Structure (by ref)"))
  (if (== OtherActor (`GameplayStatics.GetPlayerCharacter` 0))
    (`/Engine/EditorBlueprintResources/StandardMacros.DoOnce` false
      (:`Completed`
        (`GameplayStatics.PlaySound2D` "/Game/Dynamic/MetaSound/Sounds/MS_PolonezStartUp.MS_PolonezStartUp" 1.0 1.0 0.0 null null)
        (`self.DisableInput` (`GameplayStatics.GetPlayerPawn` 0) (`GameplayStatics.GetPlayerController` 0))
        (`PlayerCameraManager.StartCameraFade` :`self` (`GameplayStatics.GetPlayerCameraManager` 0) :`FromAlpha` 0.0 :`ToAlpha` 2.0 :`Duration` 3.5)
        (`KismetSystemLibrary.Delay` 3.5)
        (`self.EnableInput` (`GameplayStatics.GetPlayerPawn` 0) (`GameplayStatics.GetPlayerController` 0))
        (`GameplayStatics.OpenLevel` "MAP_Library")))))

(fn `UserConstructionScript`)