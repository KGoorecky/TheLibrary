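; BP_BathDoors is the level-one bathroom sliding door, openable once after the player has eaten pierogi.
; Hovering caches the character and toggles the interaction prompt until the bathroom is opened.
; Interacting sets the opened flag, plays an ambient sound and slides the door through a timeline.
; A parallel ChangeMusic timeline acts as a delay, then plays the after-murder ambience and flags the bath as entered.
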(event `/Game/Dynamic/Interfaces/IF_Interact.OnInteract`
  (params (InteractingPlayer :type "Character Object Reference"))
  (if (`/Game/Dynamic/Characters/LevelOne/BP_CharacterLevelOne.HasEatenPierogi` (stale `/Game/Dynamic/Interfaces/IF_Interact.OnHovered` _output_get))
    (`/Engine/EditorBlueprintResources/StandardMacros.DoOnce` false
      (:`Completed`
        (`/Game/Dynamic/UI/WB_InteractPrompt.ToggleInteractionIndicator` (`/Game/Dynamic/Characters/LevelOne/BP_CharacterLevelOne.InteractPromptWidget` (stale `/Game/Dynamic/Interfaces/IF_Interact.OnHovered` PlayerRefLevelOne)) false)
        (set `/Game/Dynamic/Characters/LevelOne/BP_CharacterLevelOne.HasOpenedBathroom` true (stale `/Game/Dynamic/Interfaces/IF_Interact.OnHovered` _output_get))
        (`|ExecutionSequence`
          (:`then_0`
            (`GameplayStatics.PlaySound2D` "/Game/Dynamic/MetaSound/Music/MS_Ambient-after-intro.MS_Ambient-after-intro" 1.0 1.0 0.0 null null)
            (bind (_direction _sliding) (`Timeline|DoorSlide`)
              (:`Update`
                (`SceneComponent.K2_SetRelativeLocation` (`self.Scene`) (`KismetMathLibrary.VLerp` (0.0 0.0 0.0) (0.0 -90.0 0.0) _sliding) false false))))
          (:`then_1`
            (`Timeline|Change Music`
              (:`Finished`
                (`GameplayStatics.PlaySound2D` "/Game/Dynamic/MetaSound/Music/MS_Ambient-after-murder.MS_Ambient-after-murder" 1.0 1.0 0.0 null null)
                (set `/Game/Dynamic/Characters/LevelOne/BP_CharacterLevelOne.HasEnteredBath` true (`self.CharacterLevelOne`))))))))))

(event `/Game/Dynamic/Interfaces/IF_Interact.OnHovered`
  (params (IsHovered :type Boolean) (PlayerRefMC :type "/Game/Dynamic/Characters/MainCharacter/BP_MainCharacter Object Reference") (PlayerRefLevelOne :type "/Game/Dynamic/Characters/LevelOne/BP_CharacterLevelOne Object Reference"))
  (bind _output_get (set `self.CharacterLevelOne` PlayerRefLevelOne))
  (if (and (`/Game/Dynamic/Characters/LevelOne/BP_CharacterLevelOne.HasEatenPierogi` _output_get) (not (`/Game/Dynamic/Characters/LevelOne/BP_CharacterLevelOne.HasOpenedBathroom` _output_get)))
    (`/Engine/EditorBlueprintResources/StandardMacros.IsValid` PlayerRefLevelOne
      (:`Is Valid`
        (`/Game/Dynamic/UI/WB_InteractPrompt.ToggleInteractionIndicator` (`/Game/Dynamic/Characters/LevelOne/BP_CharacterLevelOne.InteractPromptWidget` PlayerRefLevelOne) IsHovered)))))

(fn `IsInteractable`
  (returns (Interactable :type Boolean))
  (return false))

(fn `UserConstructionScript`)