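; BP_ScaryAhhJumscare is a one-shot audio jumpscare that triggers once the level one player character has the Piwo.
; Two collision volumes check that the overlapping actor is BP_CharacterLevelOne, then read HasPiwo from the player pawn.
; Both feed a shared DoOnce, so whichever fires first plays MS_Jumpscare at a hard-coded world location and the other stays silent.
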(event `self.JumpscareCollision1.OnComponentBeginOverlap`
  (params (OverlappedComponent :type "PrimitiveComponent Object Reference") (OtherActor :type "Actor Object Reference") (OtherComp :type "PrimitiveComponent Object Reference") (OtherBodyIndex :type Integer) (bFromSweep :type Boolean) (SweepResult :type "HitResult Structure (by ref)"))
  (if (== (`GameplayStatics.GetObjectClass` OtherActor) "/Game/Dynamic/Characters/LevelOne/BP_CharacterLevelOne.BP_CharacterLevelOne_C")
    (bind _asbp_character_level_one (cast `/Game/Dynamic/Characters/LevelOne/BP_CharacterLevelOne` (`GameplayStatics.GetPlayerPawn` 0)))
    (if (`/Game/Dynamic/Characters/LevelOne/BP_CharacterLevelOne.HasPiwo` _asbp_character_level_one)
      (`/Engine/EditorBlueprintResources/StandardMacros.DoOnce` false :!label _label
        (:`Completed`
          (`GameplayStatics.PlaySoundAtLocation` "/Game/Dynamic/MetaSound/Sounds/MS_Jumpscare.MS_Jumpscare" (-600.0 1080.0 100.0) (struct) 1.0 1.0 0.0 null null null null))))))

(event `self.JumpscareCollision2.OnComponentBeginOverlap`
  (params (OverlappedComponent :type "PrimitiveComponent Object Reference") (OtherActor :type "Actor Object Reference") (OtherComp :type "PrimitiveComponent Object Reference") (OtherBodyIndex :type Integer) (bFromSweep :type Boolean) (SweepResult :type "HitResult Structure (by ref)"))
  (if (== (`GameplayStatics.GetObjectClass` OtherActor) "/Game/Dynamic/Characters/LevelOne/BP_CharacterLevelOne.BP_CharacterLevelOne_C")
    (bind _asbp_character_level_one (cast `/Game/Dynamic/Characters/LevelOne/BP_CharacterLevelOne` (`GameplayStatics.GetPlayerPawn` 0)))
    (if (`/Game/Dynamic/Characters/LevelOne/BP_CharacterLevelOne.HasPiwo` _asbp_character_level_one)
      (goto _label))))

(fn `UserConstructionScript`)