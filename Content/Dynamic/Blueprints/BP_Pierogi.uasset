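; Pierogi interactable for level one that the player can eat once they have pierogi.
; OnInteract casts to BP_CharacterLevelOne and, behind a DoOnce, sets HasEatenPierogi, plays the pierogi sound at the actor and hides the interaction prompt.
; OnHovered toggles that prompt only while the character has pierogi and has not eaten them.
; IsInteractable always returns false.
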(event `/Game/Dynamic/Interfaces/IF_Interact.OnInteract`
  (params (InteractingPlayer :type "Character Object Reference"))
  (bind _asbp_character_level_one (cast `/Game/Dynamic/Characters/LevelOne/BP_CharacterLevelOne` InteractingPlayer))
  (bind _output_get (set `self.CharacterLevelOne` _asbp_character_level_one))
  (if (`/Game/Dynamic/Characters/LevelOne/BP_CharacterLevelOne.HasPierogi` _output_get)
    (`/Engine/EditorBlueprintResources/StandardMacros.DoOnce` false
      (:`Completed`
        (set `/Game/Dynamic/Characters/LevelOne/BP_CharacterLevelOne.HasEatenPierogi` true (`self.CharacterLevelOne`))
        (`GameplayStatics.PlaySoundAtLocation` "/Game/Dynamic/MetaSound/Sounds/MS_Pierogi.MS_Pierogi" (`self.K2_GetActorLocation`) (struct) 1.0 1.0 0.0 null null null null)
        (`/Game/Dynamic/UI/WB_InteractPrompt.ToggleInteractionIndicator` (`/Game/Dynamic/Characters/LevelOne/BP_CharacterLevelOne.InteractPromptWidget` (stale `/Game/Dynamic/Interfaces/IF_Interact.OnHovered` PlayerRefLevelOne)) false)))))

(event `/Game/Dynamic/Interfaces/IF_Interact.OnHovered`
  (params (IsHovered :type Boolean) (PlayerRefMC :type "/Game/Dynamic/Characters/MainCharacter/BP_MainCharacter Object Reference") (PlayerRefLevelOne :type "/Game/Dynamic/Characters/LevelOne/BP_CharacterLevelOne Object Reference"))
  (bind _output_get (set `self.CharacterLevelOne` PlayerRefLevelOne))
  (if (and (`/Game/Dynamic/Characters/LevelOne/BP_CharacterLevelOne.HasPierogi` _output_get) (not (`/Game/Dynamic/Characters/LevelOne/BP_CharacterLevelOne.HasEatenPierogi` _output_get)))
    (`/Engine/EditorBlueprintResources/StandardMacros.IsValid` PlayerRefLevelOne
      (:`Is Valid`
        (`/Game/Dynamic/UI/WB_InteractPrompt.ToggleInteractionIndicator` (`/Game/Dynamic/Characters/LevelOne/BP_CharacterLevelOne.InteractPromptWidget` PlayerRefLevelOne) IsHovered)))))

(fn `IsInteractable`
  (returns (Interactable :type Boolean))
  (return false))

(fn `UserConstructionScript`)