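; BP_ufotrigger is a trigger box that plays a one-time UFO cutscene when the player character overlaps it.
; It blends the view to BP_camera with a sound, lights a BP_Lightalien, starts WTFDialogue after a delay, then blends back to the player.
; A final sound accompanies switching on a BP_Leavelvl point light.
; Both light actors come from random picks among interface implementers, and a failed cast halts the sequence.
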(event `self.Box.OnComponentBeginOverlap`
  (params (OverlappedComponent :type "PrimitiveComponent Object Reference") (OtherActor :type "Actor Object Reference") (OtherComp :type "PrimitiveComponent Object Reference") (OtherBodyIndex :type Integer) (bFromSweep :type Boolean) (SweepResult :type "HitResult Structure (by ref)"))
  (if (== OtherActor (`GameplayStatics.GetPlayerCharacter` 0))
    (`/Engine/EditorBlueprintResources/StandardMacros.DoOnce` false
      (:`Completed`
        (bind _returnvalue (`GameplayStatics.GetActorOfClass` "/Game/Dynamic/Blueprints/BP_camera.BP_camera_C"))
        (`PlayerController.SetViewTargetWithBlend` (`GameplayStatics.GetPlayerController` 0) _returnvalue 3.0 "VTBlend_Linear" 2.0 false)
        (`GameplayStatics.PlaySound2D` "/Game/Dynamic/MetaSound/Sounds/MS_Ladder.MS_Ladder" 1.0 1.0 0.0 null null)
        (bind _outactors (`GameplayStatics.GetAllActorsWithInterface` "/Game/Dynamic/Interfaces/test.test_C"))
        (bind _asbp_lightalien (cast `/Game/Dynamic/Blueprints/BP_Lightalien` (`KismetArrayLibrary.Array_Random` _outactors)))
        (`SceneComponent.SetVisibility` (`/Game/Dynamic/Blueprints/BP_Lightalien.PointLight` _asbp_lightalien) true false)
        (`SceneComponent.SetVisibility` (`/Game/Dynamic/Blueprints/BP_Lightalien.SpotLight` _asbp_lightalien) true false)
        (`KismetSystemLibrary.Delay` 3.0)
        (bind _returnvalue_2 (`AddComponent|NODE_AddAC_Dialogue-0` :`self` (`GameplayStatics.GetPlayerController` 0)))
        (`/Game/Dynamic/Characters/MainCharacter/AC_Dialogue.StartDialogue` _returnvalue_2 (`self.WTFDialogue`))
        (`KismetSystemLibrary.Delay` 3.0)
        (`PlayerController.SetViewTargetWithBlend` (`GameplayStatics.GetPlayerController` 0) (`GameplayStatics.GetPlayerCharacter` 0) 2.0 "VTBlend_Linear" 1.0 false)
        (`GameplayStatics.PlaySound2D` "/Game/Dynamic/MetaSound/Sounds/MS_DescendLadder.MS_DescendLadder" 1.0 1.0 0.0 null null)
        (bind _outactors_2 (`GameplayStatics.GetAllActorsWithInterface` "/Game/Dynamic/Interfaces/test2.test2_C"))
        (bind _asbp_leavelvl (cast `/Game/Dynamic/Blueprints/BP_Leavelvl` (`KismetArrayLibrary.Array_Random` _outactors_2)))
        (`SceneComponent.SetVisibility` (`/Game/Dynamic/Blueprints/BP_Leavelvl.PointLight` _asbp_leavelvl) true false)))))

(fn `UserConstructionScript`)