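; BP_Backpack is a level-one interactable that drives a two-step backpack sequence and the transition to MAP_Library.
; Once the player has entered the bath, the first interaction shows the backpack mesh and flags it taken off, with a DoOnce/FlipFlop gating steps.
; The second swaps the mesh, plays a jumpscare sound, blends to BP_camera and fades out before loading the library.
; Hovering toggles the interaction prompt until the backpack is opened.
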(event `/Game/Dynamic/Interfaces/IF_Interact.OnInteract`
  (params (InteractingPlayer :type "Character Object Reference"))
  (bind _asbp_character_level_one (cast `/Game/Dynamic/Characters/LevelOne/BP_CharacterLevelOne` InteractingPlayer))
  (bind _output_get (set `self.CharacterLevelOne` _asbp_character_level_one))
  (if (`/Game/Dynamic/Characters/LevelOne/BP_CharacterLevelOne.HasEnteredBath` _output_get)
    (`/Engine/EditorBlueprintResources/StandardMacros.DoOnce` false :!label _label
      (:`Completed`
        (`/Engine/EditorBlueprintResources/StandardMacros.FlipFlop`
          (:`A`
            (`SceneComponent.SetVisibility` (`self.Cube`) true false)
            (set `/Game/Dynamic/Characters/LevelOne/BP_CharacterLevelOne.HasTakenOffBackpack` true _output_get)
            (`KismetSystemLibrary.Delay` 1.0)
            (goto _label :!via `Reset`))
          (:`B`
            (`StaticMeshComponent.SetStaticMesh` (`self.Cube`) "/Game/Static/Meshes/BackpackOpened/back2.back2")
            (set `/Game/Dynamic/Characters/LevelOne/BP_CharacterLevelOne.HasOpenedBackpack` true (`self.CharacterLevelOne`))
            (`/Game/Dynamic/UI/WB_InteractPrompt.ToggleInteractionIndicator` (`/Game/Dynamic/Characters/LevelOne/BP_CharacterLevelOne.InteractPromptWidget` (stale `/Game/Dynamic/Interfaces/IF_Interact.OnHovered` PlayerRefLevelOne)) false)
            (`GameplayStatics.PlaySoundAtLocation` "/Game/Dynamic/MetaSound/Sounds/MS_Jumpscare.MS_Jumpscare" (`self.K2_GetActorLocation`) (struct) 1.0 1.0 0.0 null null null null)
            (bind _returnvalue (`GameplayStatics.GetActorOfClass` "/Game/Dynamic/Blueprints/BP_camera.BP_camera_C"))
            (`PlayerController.SetViewTargetWithBlend` (`GameplayStatics.GetPlayerController` 0) _returnvalue 2.0 "VTBlend_Cubic" 0.0 false)
            (`PlayerCameraManager.StartCameraFade` :`self` (`GameplayStatics.GetPlayerCameraManager` 0) :`ToAlpha` 2.0 :`Duration` 10.0)
            (`KismetSystemLibrary.Delay` 6.0)
            (`GameplayStatics.OpenLevel` "MAP_Library")))))))

(event `/Game/Dynamic/Interfaces/IF_Interact.OnHovered`
  (params (IsHovered :type Boolean) (PlayerRefMC :type "/Game/Dynamic/Characters/MainCharacter/BP_MainCharacter Object Reference") (PlayerRefLevelOne :type "/Game/Dynamic/Characters/LevelOne/BP_CharacterLevelOne Object Reference"))
  (bind _output_get (set `self.CharacterLevelOne` PlayerRefLevelOne))
  (if (not (`/Game/Dynamic/Characters/LevelOne/BP_CharacterLevelOne.HasOpenedBackpack` _output_get))
    (`/Engine/EditorBlueprintResources/StandardMacros.IsValid` PlayerRefLevelOne
      (:`Is Valid`
        (`/Game/Dynamic/UI/WB_InteractPrompt.ToggleInteractionIndicator` (`/Game/Dynamic/Characters/LevelOne/BP_CharacterLevelOne.InteractPromptWidget` PlayerRefLevelOne) IsHovered)))))

(fn `IsInteractable`
  (returns (Interactable :type Boolean))
  (return false))

(fn `UserConstructionScript`)