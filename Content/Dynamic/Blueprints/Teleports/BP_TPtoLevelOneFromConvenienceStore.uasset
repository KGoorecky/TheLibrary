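; Interactable teleport that takes the player from the convenience store to MAP_LevelOne once they have paid for the piwo.
; Hovering caches the level-one player reference and, if HasPaidForPiwo is set, toggles that player's interaction prompt.
; Interacting checks the same flag on the cached player before opening the level by name.
; IsInteractable always returns false, so gating within this Blueprint rests on the payment flag.
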(event `/Game/Dynamic/Interfaces/IF_Interact.OnInteract`
  (params (InteractingPlayer :type "Character Object Reference"))
  (if (`/Game/Dynamic/Characters/LevelOne/BP_CharacterLevelOne.HasPaidForPiwo` (stale `/Game/Dynamic/Interfaces/IF_Interact.OnHovered` _output_get))
    (`GameplayStatics.OpenLevel` "MAP_LevelOne")))

(event `/Game/Dynamic/Interfaces/IF_Interact.OnHovered`
  (params (IsHovered :type Boolean) (PlayerRefMC :type "/Game/Dynamic/Characters/MainCharacter/BP_MainCharacter Object Reference") (PlayerRefLevelOne :type "/Game/Dynamic/Characters/LevelOne/BP_CharacterLevelOne Object Reference"))
  (bind _output_get (set `self.CharacterLevelOne` PlayerRefLevelOne))
  (if (`/Game/Dynamic/Characters/LevelOne/BP_CharacterLevelOne.HasPaidForPiwo` _output_get)
    (`/Engine/EditorBlueprintResources/StandardMacros.IsValid` PlayerRefLevelOne
      (:`Is Valid`
        (`/Game/Dynamic/UI/WB_InteractPrompt.ToggleInteractionIndicator` (`/Game/Dynamic/Characters/LevelOne/BP_CharacterLevelOne.InteractPromptWidget` PlayerRefLevelOne) IsHovered)))))

(fn `IsInteractable`
  (returns (Interactable :type Boolean))
  (return false))

(fn `UserConstructionScript`)