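; BP_TPtoApartment is an interactable teleport that sends the level-one player character to MAP_Apartment, gated on the character's HasPiwo flag (Polish for beer).
; Hovering caches the player reference and, with the flag set, toggles the interaction prompt indicator.
; Interacting marks HasEnteredApartment on both the character and GI_Instance, then opens the map by name.
; IsInteractable always returns false, leaving the gating to the events.
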(event `/Game/Dynamic/Interfaces/IF_Interact.OnInteract`
  (params (InteractingPlayer :type "Character Object Reference"))
  (if (`/Game/Dynamic/Characters/LevelOne/BP_CharacterLevelOne.HasPiwo` (stale `/Game/Dynamic/Interfaces/IF_Interact.OnHovered` _output_get))
    (set `/Game/Dynamic/Characters/LevelOne/BP_CharacterLevelOne.HasEnteredApartment` true (`self.CharacterLevelOne`))
    (bind _asgi_instance (cast `/Game/Dynamic/GI_Instance` (`GameplayStatics.GetGameInstance`)))
    (set `/Game/Dynamic/GI_Instance.HasEnteredApartment` true _asgi_instance)
    (`GameplayStatics.OpenLevel` "MAP_Apartment")))

(event `/Game/Dynamic/Interfaces/IF_Interact.OnHovered`
  (params (IsHovered :type Boolean) (PlayerRefMC :type "/Game/Dynamic/Characters/MainCharacter/BP_MainCharacter Object Reference") (PlayerRefLevelOne :type "/Game/Dynamic/Characters/LevelOne/BP_CharacterLevelOne Object Reference"))
  (bind _output_get (set `self.CharacterLevelOne` PlayerRefLevelOne))
  (if (`/Game/Dynamic/Characters/LevelOne/BP_CharacterLevelOne.HasPiwo` _output_get)
    (`/Engine/EditorBlueprintResources/StandardMacros.IsValid` PlayerRefLevelOne
      (:`Is Valid`
        (`/Game/Dynamic/UI/WB_InteractPrompt.ToggleInteractionIndicator` (`/Game/Dynamic/Characters/LevelOne/BP_CharacterLevelOne.InteractPromptWidget` PlayerRefLevelOne) IsHovered)))))

(fn `IsInteractable`
  (returns (Interactable :type Boolean))
  (return false))

(fn `UserConstructionScript`)