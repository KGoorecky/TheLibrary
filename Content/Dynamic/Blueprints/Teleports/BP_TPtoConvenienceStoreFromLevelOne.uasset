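; Interactable teleport that sends the player from Level One to the convenience store map while the character does not have piwo.
; Hovering stores the Level One character reference and toggles its interaction indicator if HasPiwo is false.
; Interacting checks the same flag, plays a door-opening sound, then loads MAP_ConvenienceStore by name after a short delay.
; IsInteractable always returns false.
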(event `self.OnInteract`
  (params (InteractingPlayer :type "Character Object Reference"))
  (if (not (`/Game/Dynamic/Characters/LevelOne/BP_CharacterLevelOne.HasPiwo` (stale `/Game/Dynamic/Interfaces/IF_Interact.OnHovered` _output_get)))
    (`GameplayStatics.PlaySoundAtLocation` "/Game/Dynamic/MetaSound/Sounds/MS_OpenDoors.MS_OpenDoors" (`self.K2_GetActorLocation`) (struct) 1.0 1.0 0.0 null null null null)
    (`KismetSystemLibrary.Delay` 0.25)
    (`GameplayStatics.OpenLevel` "MAP_ConvenienceStore")))

(event `/Game/Dynamic/Interfaces/IF_Interact.OnHovered`
  (params (IsHovered :type Boolean) (PlayerRefMC :type "/Game/Dynamic/Characters/MainCharacter/BP_MainCharacter Object Reference") (PlayerRefLevelOne :type "/Game/Dynamic/Characters/LevelOne/BP_CharacterLevelOne Object Reference"))
  (bind _output_get (set `self.CharacterLevelOne` PlayerRefLevelOne))
  (if (not (`/Game/Dynamic/Characters/LevelOne/BP_CharacterLevelOne.HasPiwo` _output_get))
    (`/Engine/EditorBlueprintResources/StandardMacros.IsValid` PlayerRefLevelOne
      (:`Is Valid`
        (`/Game/Dynamic/UI/WB_InteractPrompt.ToggleInteractionIndicator` (`/Game/Dynamic/Characters/LevelOne/BP_CharacterLevelOne.InteractPromptWidget` PlayerRefLevelOne) IsHovered)))))

(fn `IsInteractable`
  (returns (Interactable :type Boolean))
  (return false))

(fn `UserConstructionScript`)