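; BP_Detective-Standing is a standing detective NPC whose visibility is driven by game state.
; On BeginPlay it caches GI_Instance, sets mesh visibility from its DetectiveVisibility flag, and enables capsule collision if visible.
; A SetVisibility event toggles the mesh but always enables collision, and does not write the flag back to the game instance.
; IsInteractable always returns false.
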(event `self.ReceiveBeginPlay`
  (bind _asgi_instance (cast `/Game/Dynamic/GI_Instance` (`GameplayStatics.GetGameInstance`)))
  (bind _output_get (set `self.Game Instance` _asgi_instance))
  (bind _detectivevisibility (`/Game/Dynamic/GI_Instance.DetectiveVisibility` _output_get))
  (`SceneComponent.SetVisibility` (`self.Mesh`) _detectivevisibility false)
  (if _detectivevisibility
    (`PrimitiveComponent.SetCollisionEnabled` (`self.CapsuleComponent`) "QueryAndPhysics")))

(event `/Game/Dynamic/Interfaces/IF_Interact.SetVisibility`
  (params (Visibility :type Boolean))
  (`SceneComponent.SetVisibility` (`self.Mesh`) Visibility false)
  (`PrimitiveComponent.SetCollisionEnabled` (`self.CapsuleComponent`) "QueryAndPhysics")
  (cast `/Game/Dynamic/GI_Instance` (`GameplayStatics.GetGameInstance`)))

(fn `IsInteractable`
  (returns (Interactable :type Boolean))
  (return false))

(fn `UserConstructionScript`)