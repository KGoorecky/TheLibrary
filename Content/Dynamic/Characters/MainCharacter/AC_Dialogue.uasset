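; Dialogue component in the main character folder that plays a sequence of lines from a data table with on-screen text and audio.
; StartDialogue creates the WB_Dialogue widget and caches the table's row names, then NextDialogue shows each row's speaker and text, plays its sound and waits for its Length.
; This Delay-driven loop ends by removing the widget; Counter is never reset here, and the cleared Timer handle is never set to a timer.
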(event `StartDialogue`
  (params (Dialogues :type "DataTable Object Reference"))
  ;[0 0 0] Start Dialogue
  (set `self.DialoguesTable` Dialogues)
  (bind _returnvalue (`|CreateWidget` "/Game/Dynamic/UI/WB_Dialogue.WB_Dialogue_C" (`GameplayStatics.GetPlayerController` 0)))
  (bind _output_get (set `self.DialogueWidget` _returnvalue))
  (`UserWidget.AddToViewport` _output_get 0)
  (`self.Setup Dialogue`)
  (`self.Next Dialogue`)
  (set `self.Timer` (struct)))

(event `Next Dialogue`
  (bind _dialoguewidget (`self.DialogueWidget`))
  ;[0 0 0] Next Dialogue
  (if (!= (`self.Counter`) (`KismetArrayLibrary.Array_Length` (`self.RowNames`))) :!label _label
    (bind _returnvalue (`|GetDataTableRow` (`self.DialoguesTable`) (`|GetArrayItem` (`self.RowNames`) (`self.Counter`)))
      (:`then`
        (bind (_name _text _audio _length) (break `/Game/Dynamic/Structures/S_Dialogue` _returnvalue))
        (`/Game/Dynamic/UI/WB_Dialogue.UpdateName` _dialoguewidget (`KismetTextLibrary.Conv_StringToText` (`KismetStringLibrary.Concat_StrStr` _name ": ")))
        (`/Game/Dynamic/UI/WB_Dialogue.UpdateText` _dialoguewidget (`KismetTextLibrary.Conv_StringToText` _text))
        (`GameplayStatics.PlaySound2D` _audio 1.0 1.0 0.0 null null)
        (`/Engine/EditorBlueprintResources/StandardMacros.IncrementInt` (`self.Counter`)
          (:`  `
            (`KismetSystemLibrary.Delay` _length)
            (goto _label)))))
    (else
      (`self.End Dialogue`))))

(event `Setup Dialogue`
  ;[0 0 0] Setup Dialogue
  (bind _outrownames (`DataTableFunctionLibrary.GetDataTableRowNames` (`self.DialoguesTable`)))
  (set `self.RowNames` _outrownames))

(event `End Dialogue`
  ;[0 0 0] End Dialogue
  (`KismetSystemLibrary.K2_ClearAndInvalidateTimerHandle` (`self.Timer`))
  (`Widget.RemoveFromParent` (`self.DialogueWidget`)))